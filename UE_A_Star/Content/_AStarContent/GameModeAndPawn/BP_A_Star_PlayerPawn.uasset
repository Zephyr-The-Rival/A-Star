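; Player pawn for an A* pathfinding scene that lets the mouse edit grid tiles or set the agent's goal.
; BeginPlay shows the cursor and creates the HUD.
; Left click traces under the cursor and, by CursorMode, toggles a BP_Tile's walkability or sends a walkable tile to BP_Agent.
; Tick resets the last tile's glow and colors the hovered tile's edges by mode and walkability; ClickingBlocked suspends clicking and hovering.
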(event EventBeginPlay
  (bind _returnvalue (Game|GetPlayerController 0))
  (Variables|/Script/Engine.PlayerController|SetbShowMouseCursor _returnvalue true)
  (Input|SetInputModeGameandUI _returnvalue 0 "DoNotLock" false false)
  (bind _returnvalue_2 (UserInterface|CreateWidget "/Game/_AStarContent/GameModeAndPawn/PlayerHud.PlayerHud_C"))
  (UserInterface|Viewport|AddtoViewport _returnvalue_2 0))

(event Collision|EventActorBeginOverlap
  (params (OtherActor :type Actor%20Object%20Reference)))

(event EventTick
  (params (DeltaSeconds :type Float%20%28single-precision%29))
  (Utilities|FlowControl|Sequence
    (:then_0
      (Utilities|IsValid (Variables|Default|GetCurrentHighlightedTile)
        (:Is%20Valid
          (Rendering|Material|SetVectorParameterValue (Variables|/Game/_AStarContent/Grid/BP_Tile.BP_Tile_C|GetDynamicMaterial (Variables|Default|GetCurrentHighlightedTile)) "GlowColor" "(R=0.010000,G=0.010000,B=0.010000,A=1.000000)" :!class /Script/Engine.MaterialInstanceDynamic))))
    (:then_1
      (if (not (Variables|Default|GetClickingBlocked))
        (bind _asbp_tile (Utilities|Casting|CastToBP_Tile (.HitActor (Collision|BreakHitResult (.HitResult (Game|Player|GetHitResultUnderCursorbyChannel (Game|GetPlayerController 0) "TraceTypeQuery1" true))))))
        (switch Utilities|FlowControl|Switch|SwitchonClickModes (Variables|Default|GetCursorMode)
          (:NewEnumerator0
            (if (Variables|/Game/_AStarContent/Grid/BP_Tile.BP_Tile_C|GetWalkable _asbp_tile)
              (Default|SetEdgesColor _asbp_tile "(R=1.000000,G=0.012164,B=0.000000,A=30.000000)")
              (Variables|Default|SetCurrentHighlightedTile _asbp_tile)
              (else
                (Default|SetEdgesColor _asbp_tile "(R=0.000000,G=0.511214,B=1.000000,A=30.000000)")
                (Variables|Default|SetCurrentHighlightedTile _asbp_tile))))
          (:NewEnumerator1
            (Default|SetEdgesColor _asbp_tile "(R=0.322035,G=1.000000,B=0.000000,A=30.000000)")
            (Variables|Default|SetCurrentHighlightedTile _asbp_tile)))))))

(event Input|MouseEvents|LeftMouseButton
  (params (Key :type Key%20Structure :default "None"))
  (bind _returnvalue (Game|GetPlayerController 0))
  (bind (_hitresult _returnvalue_2) (Game|Player|GetHitResultUnderCursorbyChannel _returnvalue "TraceTypeQuery1" true))
  (:Pressed
    (if (not (Variables|Default|GetClickingBlocked))
      (if _returnvalue_2
        (bind _asbp_tile (Utilities|Casting|CastToBP_Tile (.HitActor (Collision|BreakHitResult _hitresult))))
        (switch Utilities|FlowControl|Switch|SwitchonClickModes (Variables|Default|GetCursorMode)
          (:NewEnumerator0
            (Default|ToggleWalkable _asbp_tile))
          (:NewEnumerator1
            (if (Variables|/Game/_AStarContent/Grid/BP_Tile.BP_Tile_C|GetWalkable _asbp_tile)
              (bind _returnvalue_3 (Actor|GetActorOfClass "/Game/_AStarContent/Agent/BP_Agent.BP_Agent_C"))
              (Default|SetNewGoal _returnvalue_3 _asbp_tile))))))))

(fn ConstructionScript)

(fn SetClickingBlocked
  (params (ClickingBlocked :type Boolean))
  (Variables|Default|SetClickingBlocked ClickingBlocked))