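; Grid tile actor for A* pathfinding that stores walkability and path costs.
; Finds neighbors through BP_Grid, allowing diagonals only when both adjacent orthogonal tiles are walkable.
; CalculateCosts sums accumulated distance from start and straight-line distance to goal, keeping and displaying improved totals.
; Toggling walkability animates the plane's height via timelines, while a dynamic material drives base and edge glow colors.
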(event Custom|ToggleWalkable
  (bind _plane (Variables|Default|GetPlane))
  (bind _plane_2 (Variables|Default|GetPlane))
  (bind _returnvalue (Transformation|GetWorldLocation _plane))
  (bind _returnvalue_2 (Transformation|GetWorldLocation _plane_2))
  (if (not (Variables|Default|GetToggleInProgress))
    (Variables|Default|SetToggleInProgress true)
    (if (Variables|Default|GetWalkable)
      (Variables|Default|SetWalkable false)
      (CallFunction|SetColor (Math|Color|MakeColor 10 10 10 255))
      (bind _0_to_100 (Timeline|MoveTileDown PlayFromStart)
        (:Update
          (Transformation|SetWorldLocation _plane_2 (Math|Vector|MakeVector (.x _returnvalue_2) (.y _returnvalue_2) _0_to_100) false false))
        (:Finished
          (Variables|Default|SetToggleInProgress false)))
      (else
        (bind _100_to_0 (Timeline|Timeline PlayFromStart)
          (:Update
            (Transformation|SetWorldLocation _plane (Math|Vector|MakeVector (.x _returnvalue) (.y _returnvalue) _100_to_0) false false))
          (:Finished
            (Variables|Default|SetWalkable true)
            (Variables|Default|SetToggleInProgress false)
            (CallFunction|ResetColor)))))))

(event EventBeginPlay)

(event EventTick
  (params (DeltaSeconds :type Float%20%28single-precision%29)))

(fn ConstructionScript
  (bind _returnvalue (Rendering|Material|CreateDynamicMaterialInstance (Variables|Default|GetPlane) 0 "/Game/_AStarContent/Materials/TileMaterial.TileMaterial" "None" :!class /Script/Engine.PrimitiveComponent))
  (Variables|Default|SetDynamicMaterial _returnvalue)
  (CallFunction|ResetColor)
  (Rendering|Material|SetVectorParameterValue (Variables|Default|GetDynamicMaterial) "GlowColor" "(R=0.010000,G=0.010000,B=0.010000,A=1.000000)" :!class /Script/Engine.MaterialInstanceDynamic))

(fn SetColor
  (params (NewColor :type Color%20Structure))
  (Rendering|Material|SetVectorParameterValue (Variables|Default|GetDynamicMaterial) "Base Color" (Math|Conversions|ToLinearColor(Color) NewColor) :!class /Script/Engine.MaterialInstanceDynamic))

(fn GetNeighbor
  (params (Direction :type Directions%20Enum :default "NewEnumerator0"))
  (Utilities|FlowControl|Sequence
    (:then_0
      (bind _returnvalue (Actor|GetActorOfClass "/Game/_AStarContent/Grid/BP_Grid.BP_Grid_C"))
      (LocalVariables|SetLocal%20Grid _returnvalue))
    (:then_1
      (switch Utilities|FlowControl|Switch|SwitchonDirections Direction
        (:NewEnumerator0
          (return (Default|GetTile (LocalVariables|GetLocal%20Grid) (+ (Variables|Default|GetMyRow) 1) (Variables|Default|GetMyColum))))
        (:NewEnumerator1
          (return (Default|GetTile (LocalVariables|GetLocal%20Grid) (+ (Variables|Default|GetMyRow) -1) (Variables|Default|GetMyColum))))
        (:NewEnumerator2
          (return (Default|GetTile (LocalVariables|GetLocal%20Grid) (Variables|Default|GetMyRow) (+ (Variables|Default|GetMyColum) -1))))
        (:NewEnumerator3
          (return (Default|GetTile (LocalVariables|GetLocal%20Grid) (Variables|Default|GetMyRow) (+ (Variables|Default|GetMyColum) 1))))
        (:NewEnumerator4
          (return (Default|GetTile (LocalVariables|GetLocal%20Grid) (+ (Variables|Default|GetMyRow) 1) (+ (Variables|Default|GetMyColum) -1))))
        (:NewEnumerator5
          (return (Default|GetTile (LocalVariables|GetLocal%20Grid) (+ (Variables|Default|GetMyRow) 1) (+ (Variables|Default|GetMyColum) 1))))
        (:NewEnumerator6
          (return (Default|GetTile (LocalVariables|GetLocal%20Grid) (+ (Variables|Default|GetMyRow) -1) (+ (Variables|Default|GetMyColum) -1))))
        (:NewEnumerator7
          (return (Default|GetTile (LocalVariables|GetLocal%20Grid) (+ (Variables|Default|GetMyRow) -1) (+ (Variables|Default|GetMyColum) 1))))))))

(fn GetAllWalkableNeighbors
  (bind _selectedneighbor (CallFunction|GetNeighbor "NewEnumerator5"))
  (bind _selectedneighbor_2 (CallFunction|GetNeighbor "NewEnumerator6"))
  (bind _selectedneighbor_3 (CallFunction|GetNeighbor "NewEnumerator7"))
  (bind _selectedneighbor_4 (CallFunction|GetNeighbor "NewEnumerator4"))
  (Utilities|FlowControl|Sequence
    (:then_0
      (for _index (range 0 3)
        (if (Utilities|IsValid (CallFunction|GetNeighbor (Utilities|Enum|ByteToEnumDirections (Math|Conversions|ToByte(Integer) _index))))
          (if (Variables|BP_Tile_C|GetWalkable (CallFunction|GetNeighbor (Utilities|Enum|ByteToEnumDirections (Math|Conversions|ToByte(Integer) _index))))
            (Utilities|Array|Add (LocalVariables|GetNeignbors%20Local) (CallFunction|GetNeighbor (Utilities|Enum|ByteToEnumDirections (Math|Conversions|ToByte(Integer) _index))))))))
    (:then_1
      (Utilities|FlowControl|Sequence
        (:then_0
          (Utilities|IsValid _selectedneighbor_4
            (:Is%20Valid
              (if (Math|Boolean|ANDBoolean (Variables|BP_Tile_C|GetWalkable _selectedneighbor_4) (Variables|BP_Tile_C|GetWalkable (CallFunction|GetNeighbor "NewEnumerator0")) (Variables|BP_Tile_C|GetWalkable (CallFunction|GetNeighbor "NewEnumerator2")))
                (Utilities|Array|Add (LocalVariables|GetNeignbors%20Local) _selectedneighbor_4)))))
        (:then_1
          (Utilities|IsValid _selectedneighbor
            (:Is%20Valid
              (if (Math|Boolean|ANDBoolean (Variables|BP_Tile_C|GetWalkable _selectedneighbor) (Variables|BP_Tile_C|GetWalkable (CallFunction|GetNeighbor "NewEnumerator0")) (Variables|BP_Tile_C|GetWalkable (CallFunction|GetNeighbor "NewEnumerator3")))
                (Utilities|Array|Add (LocalVariables|GetNeignbors%20Local) _selectedneighbor)))))
        (:then_2
          (Utilities|IsValid _selectedneighbor_2
            (:Is%20Valid
              (if (Math|Boolean|ANDBoolean (Variables|BP_Tile_C|GetWalkable _selectedneighbor_2) (Variables|BP_Tile_C|GetWalkable (CallFunction|GetNeighbor "NewEnumerator1")) (Variables|BP_Tile_C|GetWalkable (CallFunction|GetNeighbor "NewEnumerator2")))
                (Utilities|Array|Add (LocalVariables|GetNeignbors%20Local) _selectedneighbor_2)))))
        (:then_3
          (Utilities|IsValid _selectedneighbor_3
            (:Is%20Valid
              (if (Math|Boolean|ANDBoolean (Variables|BP_Tile_C|GetWalkable _selectedneighbor_3) (Variables|BP_Tile_C|GetWalkable (CallFunction|GetNeighbor "NewEnumerator1")) (Variables|BP_Tile_C|GetWalkable (CallFunction|GetNeighbor "NewEnumerator3")))
                (Utilities|Array|Add (LocalVariables|GetNeignbors%20Local) _selectedneighbor_3)))))))
    (:then_2
      (return (LocalVariables|GetNeignbors%20Local)))))

(fn CalculateCosts
  (params (PreviousInPath :type BP%20Tile%20Object%20Reference) (Goal :type BP%20Tile%20Object%20Reference))
  (LocalVariables|SetLocalDistanceToStart (+ (Variables|BP_Tile_C|GetDistanceToStart PreviousInPath) (Math|Vector|Distance(Vector) (Transformation|GetWorldLocation (Variables|BP_Tile_C|GetPlane PreviousInPath)) (Transformation|GetWorldLocation (Variables|Default|GetPlane)))))
  (LocalVariables|SetLocalDistanceToGoal (Math|Vector|Distance(Vector) (Transformation|GetWorldLocation (Variables|BP_Tile_C|GetPlane Goal)) (Transformation|GetWorldLocation (Variables|Default|GetPlane))))
  (if (or (< (+ (LocalVariables|GetLocalDistanceToStart) (LocalVariables|GetLocalDistanceToGoal)) (Variables|Pathfinding|GetSumCost)) (== (Variables|Pathfinding|GetSumCost) 0.0))
    (Variables|Pathfinding|SetDistanceToGoal (LocalVariables|GetLocalDistanceToGoal))
    (Variables|Pathfinding|SetDistanceToStart (LocalVariables|GetLocalDistanceToStart))
    (Variables|Pathfinding|SetSumCost (+ (LocalVariables|GetLocalDistanceToStart) (LocalVariables|GetLocalDistanceToGoal)))
    (CallFunction|DisplayCosts)
    (return true)
    (else
      (return false))))

(fn DisplayCosts
  (bind _cost (Variables|Default|GetCost))
  ;[1 1 1] Display Nuimber
  (Rendering|Components|TextRender|SetText (Variables|Default|GetDToGoal) (Utilities|Text|ToText(Float) (Variables|Pathfinding|GetDistanceToGoal) "HalfToEven" false true 1 324 0 0))
  (Rendering|Components|TextRender|SetText (Variables|Default|GetDToStart) (Utilities|Text|ToText(Float) (Variables|Pathfinding|GetDistanceToStart) "HalfToEven" false true 1 324 0 0))
  (Rendering|Components|TextRender|SetText _cost (Utilities|Text|ToText(Float) (Variables|Pathfinding|GetSumCost) "HalfToEven" false true 1 324 0 0))
  (Development|SetHiddeninGame _cost (== (Variables|Pathfinding|GetSumCost) 0.0) false))

(fn Reset
  (Variables|Pathfinding|SetSumCost 0.0)
  (Variables|Pathfinding|SetDistanceToGoal 0.0)
  (Variables|Pathfinding|SetDistanceToStart 0.0)
  (CallFunction|DisplayCosts)
  (if (Variables|Default|GetWalkable)
    (CallFunction|ResetColor)))

(fn ResetColor
  (CallFunction|SetColor (Math|Color|MakeColor 150 150 150 255)))

(fn SetEdgesColor
  (params (Color :type Linear%20Color%20Structure))
  (Rendering|Material|SetVectorParameterValue (Variables|Default|GetDynamicMaterial) "GlowColor" Color :!class /Script/Engine.MaterialInstanceDynamic))