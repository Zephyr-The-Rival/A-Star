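; BP_Grid is an actor that builds a grid of BP_Tile actors, likely for A* pathfinding.
; Its construction script adds child actor tiles spaced and scaled by TileSize, records each one's row and column, and stores them in a flat Tiles array.
; GetTile bounds-checks and looks up tiles by Row * GridRows + Colum, which matches the storage order only when row and column counts are equal.
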(event EventBeginPlay)

(event Collision|EventActorBeginOverlap
  (params (OtherActor :type Actor%20Object%20Reference)))

(event EventTick
  (params (DeltaSeconds :type Float%20%28single-precision%29)))

(fn ConstructionScript
  (bind _defaultsceneroot (Variables|Default|GetDefaultSceneRoot))
  (bind _tilesize (Variables|Default|GetTileSize))
  (bind _returnvalue (Transformation|GetWorldLocation _defaultsceneroot))
  (bind _returnvalue_2 (* _tilesize 1e+02))
  (for _index (range 0 (- (Variables|Default|GetGridRows) 1))
    (for _index_2 (range 0 (- (Variables|Default|GetGridColums) 1))
      (bind _returnvalue_3 (AddComponent|AddChildActorComponent false (Math|Transform|MakeTransform (Math|Vector|MakeVector (+ (.x _returnvalue) (* _returnvalue_2 _index)) (+ (.y _returnvalue) (* _returnvalue_2 _index_2)) 0.0) "0, 0, 0" "1.000000,1.000000,1.000000")))
      (Transformation|SetRelativeScale3D (Variables|/Game/_AStarContent/Grid/BP_Tile.BP_Tile_C|GetPlane (.AsBP%20Tile (Utilities|Casting|CastToBP_Tile (Variables|/Script/Engine.ChildActorComponent|GetChildActor _returnvalue_3)))) (Math|Conversions|ToVector(Float) (Variables|Default|GetTileSize)))
      (Utilities|Array|Add (Variables|Default|GetTiles) (.AsBP%20Tile (Utilities|Casting|CastToBP_Tile (Variables|/Script/Engine.ChildActorComponent|GetChildActor _returnvalue_3))))
      (Variables|/Game/_AStarContent/Grid/BP_Tile.BP_Tile_C|SetMyRow (.AsBP%20Tile (Utilities|Casting|CastToBP_Tile (Variables|/Script/Engine.ChildActorComponent|GetChildActor _returnvalue_3))) _index)
      (Variables|/Game/_AStarContent/Grid/BP_Tile.BP_Tile_C|SetMyColum (.AsBP%20Tile (Utilities|Casting|CastToBP_Tile (Variables|/Script/Engine.ChildActorComponent|GetChildActor _returnvalue_3))) _index_2))))

(fn GetTile
  (params (Row :type Integer) (Colum :type Integer))
  (bind _tiles (Variables|Default|GetTiles))
  (bind _gridrows (Variables|Default|GetGridRows))
  (bind _returnvalue (* Row _gridrows))
  (bind _returnvalue_2 (+ _returnvalue Colum))
  (if (Math|Boolean|ANDBoolean (Utilities|Array|IsValidIndex _tiles _returnvalue_2) (< Colum (Variables|Default|GetGridColums)) (>= Colum 0))
    (return (Utilities|Array|Get(acopy) _tiles _returnvalue_2))
    (else
      (return 0))))