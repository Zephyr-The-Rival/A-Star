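; BP_Agent is a grid agent that walks tile to tile along a path from the Pathfinder actor, starting on a BP_Grid tile.
; SetNewGoal blocks player pawn clicking, gets the path, colors its tiles red and starts the first step.
; Tick moves the agent toward ShortTermGoal at WalkingSpeed, snaps on arrival and pops the next tile.
; When the path is empty, it changes State and unblocks clicking.
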(event Custom|Go%20to%20next%20short%20term%20goal
  (bind _path (Variables|Default|GetPath))
  (if (Utilities|Array|IsValidIndex _path)
    (Variables|Default|SetShortTermGoal (Utilities|Array|Get(acopy) _path))
    (Utilities|Array|RemoveIndex _path)
    (else
      (Variables|Default|SetState "NewEnumerator0")
      (Default|SetClickingBlocked (.AsBP%20A%20Star%20Player%20Pawn (Utilities|Casting|CastToBP_A_Star_PlayerPawn (Game|Player|GetPlayerPawn 0))) false))))

(event EventBeginPlay
  ;[1 1 1] Sets the agent to the 0;0 tille
  (bind _returnvalue (Actor|GetActorOfClass "/Game/_AStarContent/Grid/BP_Grid.BP_Grid_C"))
  (bind _output_get (Variables|Default|SetCurrentTile (Default|GetTile _returnvalue 1 1)))
  (Transformation|SetWorldLocation (Variables|Default|GetDefaultSceneRoot) (Transformation|GetWorldLocation (Variables|/Game/_AStarContent/Grid/BP_Tile.BP_Tile_C|GetPlane _output_get)) false true))

(event EventTick
  (params (DeltaSeconds :type Float%20%28single-precision%29))
  (bind _defaultsceneroot (Variables|Default|GetDefaultSceneRoot))
  (bind _shorttermgoal (Variables|Default|GetShortTermGoal))
  (bind _returnvalue (Transformation|GetWorldLocation _defaultsceneroot))
  (bind _plane (Variables|/Game/_AStarContent/Grid/BP_Tile.BP_Tile_C|GetPlane _shorttermgoal))
  (bind _returnvalue_2 (Transformation|GetWorldLocation _plane))
  (bind _returnvalue_3 (- _returnvalue_2 _returnvalue))
  (if (and (Utilities|IsValid (Variables|Default|GetShortTermGoal)) (!= (Variables|Default|GetShortTermGoal) (Variables|Default|GetCurrentTile)))
    (Variables|Default|SetState "NewEnumerator1")
    ;[1 1 1] Snap to target on arrival
    (if (< (Math|Float|Absolute(Float) (Math|Vector|VectorLength _returnvalue_3)) 5.0)
      (Transformation|SetWorldLocation (Variables|Default|GetDefaultSceneRoot) (Transformation|GetWorldLocation (Variables|/Game/_AStarContent/Grid/BP_Tile.BP_Tile_C|GetPlane (Variables|Default|GetShortTermGoal))) false true)
      (Variables|Default|SetCurrentTile (Variables|Default|GetShortTermGoal))
      (CallFunction|GotoNextShortTermGoal)
      (else
        ;[1 1 1] Move Agent
        (Transformation|AddWorldOffset _defaultsceneroot (* (Math|Vector|Normalize _returnvalue_3) (Utilities|Time|GetWorldDeltaSeconds) (Variables|Default|GetWalkingSpeed)) false false)))))

(fn ConstructionScript)

(fn AddShortTermGoal
  (params (NewGoal :type BP%20Tile%20Object%20Reference))
  (Utilities|Array|Add (Variables|Default|GetPath) NewGoal)
  (if (Utilities|Enum|Equal(Enum) (Variables|Default|GetState) "NewEnumerator0")
    (CallFunction|GotoNextShortTermGoal)))

(fn SetNewGoal
  (params (NewGoal :type BP%20Tile%20Object%20Reference))
  (Default|SetClickingBlocked (.AsBP%20A%20Star%20Player%20Pawn (Utilities|Casting|CastToBP_A_Star_PlayerPawn (Game|Player|GetPlayerPawn 0))) true)
  (bind _returnvalue (Actor|GetActorOfClass "/Game/_AStarContent/Pathfinder.Pathfinder_C"))
  (Utilities|IsValid _returnvalue
    (:Is%20Valid
      (bind _path (Default|FindPath _returnvalue (Variables|Default|GetCurrentTile) NewGoal))
      (bind _output_get (Variables|Default|SetPath _path))
      (for _array_element _output_get
        (Default|SetColor _array_element (Math|Color|MakeColor 0 0 255 255)))
      (CallFunction|GotoNextShortTermGoal))
    (:Is%20Not%20Valid
      (Development|PrintString "No pathfinder found"))))